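; Player test character that fires one of three weapon types on the Fire input, selected by AmmoType.
; Hitscan line-traces along the active camera's forward vector from the aim camera and damages BP_EnemyBase hits.
; Projectile and Bomb spawn their actors at the Scene component and launch them along that vector.
; Each shot plays a sound, spends its own ammo and blocks firing through a Reloading flag for a per-weapon delay.
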(event `InputAction|Fire`
  (params (Key :type "Key Structure"))
  (bind _returnvalue (`SceneComponent.K2_GetComponentLocation` (`self.FollowCameraAim`)))
  (:`Pressed`
    (if (not (`self.bReloading`))
      (switch `EAmmoType` (`self.AmmoType`)
        (:`EAT_HitScan`
          (if (> (`self.HitScanAmmo`) 0)
            (bind _outhit (`KismetSystemLibrary.LineTraceSingle` :`Start` _returnvalue :`End` (+ _returnvalue (* (`SceneComponent.GetForwardVector` (`self.GetActiveCamera`)) 3000.0)) :`TraceChannel` "TraceTypeQuery1" :`DrawDebugType` "ForDuration" :`DrawTime` 2.0))
            (`GameplayStatics.PlaySound2D` null 1.0 1.0 0.0 null null)
            (bind _asbp_enemy_base (cast `/Game/JoyWay/Core/Enemy/BP_EnemyBase` (`.HitActor` (`GameplayStatics.BreakHitResult` _outhit)))
              (:`then`
                (`/Game/JoyWay/Core/Enemy/BP_EnemyBase.getDamage` _asbp_enemy_base 80.0))
              (:`CastFailed`
                _))
            (`/Engine/EditorBlueprintResources/StandardMacros.DecrementInt` (`self.HitScanAmmo`)
              (:`  `
                (set `self.bReloading` true)
                (`KismetSystemLibrary.Delay` 2.0)
                (set `self.bReloading` false)))))
        (:`EAT_Projectile`
          (if (> (`self.ProjectileAmmo`) 0)
            (bind _returnvalue_2 (`|SpawnActorFromClass` "/Game/JoyWay/Core/Projectiles/BP_Projectile.BP_Projectile_C" (`SceneComponent.K2_GetComponentToWorld` (`self.Scene`)) "Undefined" "OverrideRootScale" null null))
            (`GameplayStatics.PlaySound2D` null 1.0 1.0 0.0 null null)
            (`Projectile.FireInDirection` _returnvalue_2 (`SceneComponent.GetForwardVector` (`self.GetActiveCamera`)))
            (`/Engine/EditorBlueprintResources/StandardMacros.DecrementInt` (`self.ProjectileAmmo`)
              (:`  `
                (set `self.bReloading` true)
                (`KismetSystemLibrary.Delay` 0.25)
                (set `self.bReloading` false)))))
        (:`EAT_Bombing`
          (if (> (`self.BombAmmo`) 0)
            (bind _returnvalue_3 (`|SpawnActorFromClass` "/Game/JoyWay/Core/Projectiles/BP_Bomb.BP_Bomb_C" (`SceneComponent.K2_GetComponentToWorld` (`self.Scene`)) "Undefined" "OverrideRootScale" null null))
            (`GameplayStatics.PlaySound2D` null 1.0 1.0 0.0 null null)
            (`Projectile.FireInDirection` _returnvalue_3 (`SceneComponent.GetForwardVector` (`self.GetActiveCamera`)))
            (`/Engine/EditorBlueprintResources/StandardMacros.DecrementInt` (`self.BombAmmo`)
              (:`  `
                (set `self.bReloading` true)
                (`KismetSystemLibrary.Delay` 0.75)
                (set `self.bReloading` false)))))))))

(fn `UserConstructionScript`)