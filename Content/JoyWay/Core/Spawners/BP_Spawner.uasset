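; Spawner actor that populates the level with one weapon and one enemy per ammo type (HitScan, Projectile, Bombing).
; On BeginPlay it runs both spawn events and sets up a WidgetSpawner on its widget component, passing itself as the owning spawner.
; Each type spawns at its own scene component only if the tracked weapon or enemy array lacks that AmmoType.
; Spawned actors receive a reference back to the spawner.
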(event `self.ReceiveBeginPlay`
  (bind _returnvalue (`|CreateWidget` "/Game/JoyWay/Core/Spawners/WidgetSpawner.WidgetSpawner_C" null self))
  (set `self.WidgetParameter` _returnvalue)
  (`self.SpawnWeapons`)
  (`self.SpawnEnemies`)
  (`WidgetComponent.SetWidget` (`self.Widget`) (`self.WidgetParameter`)))

(event `SpawnWeapons`
  (`|ExecutionSequence`
    (:`then_0`
      (bind _found (`self.CheckForSpawnWeaponAbility` "EAT_HitScan"))
      (if (not _found)
        (bind _returnvalue (`|SpawnActorFromClass` "/Game/JoyWay/Core/Items/BP_HitscanWeapon.BP_HitscanWeapon_C" (`SceneComponent.K2_GetComponentToWorld` (`self.Scene`)) "Undefined" "OverrideRootScale" null self null))
        (`KismetArrayLibrary.Array_Add` (`self.WeaponsSpawned`) _returnvalue)))
    (:`then_1`
      (bind _found_2 (`self.CheckForSpawnWeaponAbility` "EAT_Projectile"))
      (if (not _found_2)
        (bind _returnvalue_2 (`|SpawnActorFromClass` "/Game/JoyWay/Core/Items/BP_ProjectileWeapon.BP_ProjectileWeapon_C" (`SceneComponent.K2_GetComponentToWorld` (`self.Scene1`)) "Undefined" "OverrideRootScale" null self null))
        (`KismetArrayLibrary.Array_Add` (`self.WeaponsSpawned`) _returnvalue_2)))
    (:`then_2`
      (bind _found_3 (`self.CheckForSpawnWeaponAbility` "EAT_Bombing"))
      (if (not _found_3)
        (bind _returnvalue_3 (`|SpawnActorFromClass` "/Game/JoyWay/Core/Items/BP_BombWeapon.BP_BombWeapon_C" (`SceneComponent.K2_GetComponentToWorld` (`self.Scene2`)) "Undefined" "OverrideRootScale" null self null))
        (`KismetArrayLibrary.Array_Add` (`self.WeaponsSpawned`) _returnvalue_3)))))

(event `SpawnEnemies`
  (bind _returnvalue (enumliteral `EAmmoType` "EAT_Bombing"))
  (bind _returnvalue_2 (enumliteral `EAmmoType` "EAT_HitScan"))
  (bind _returnvalue_3 (enumliteral `EAmmoType` "EAT_Projectile"))
  (`|ExecutionSequence`
    (:`then_0`
      (bind _found (`self.CheckForSpawnEnemyAbility` _returnvalue_2))
      (if (not _found)
        (bind _returnvalue_4 (`|SpawnActorFromClass` "/Game/JoyWay/Core/Enemy/BP_EnemyBase.BP_EnemyBase_C" (`SceneComponent.K2_GetComponentToWorld` (`self.Scene3`)) "Undefined" "OverrideRootScale" null self _returnvalue_2 null))
        (`KismetArrayLibrary.Array_Add` (`self.Enemies`) _returnvalue_4)))
    (:`then_1`
      (bind _found_2 (`self.CheckForSpawnEnemyAbility` _returnvalue_3))
      (if (not _found_2)
        (bind _returnvalue_5 (`|SpawnActorFromClass` "/Game/JoyWay/Core/Enemy/BP_EnemyBase.BP_EnemyBase_C" (`SceneComponent.K2_GetComponentToWorld` (`self.Scene4`)) "Undefined" "OverrideRootScale" null self _returnvalue_3 null))
        (`KismetArrayLibrary.Array_Add` (`self.Enemies`) _returnvalue_5)))
    (:`then_2`
      (bind _found_3 (`self.CheckForSpawnEnemyAbility` _returnvalue))
      (if (not _found_3)
        (bind _returnvalue_6 (`|SpawnActorFromClass` "/Game/JoyWay/Core/Enemy/BP_EnemyBase.BP_EnemyBase_C" (`SceneComponent.K2_GetComponentToWorld` (`self.Scene5`)) "Undefined" "OverrideRootScale" null self _returnvalue null))
        (`KismetArrayLibrary.Array_Add` (`self.Enemies`) _returnvalue_6)))))

(fn `CheckForSpawnEnemyAbility`
  (params (AmmoType :type "EAmmoType Enum" :default "EAT_HitScan"))
  (returns (Found :type Boolean))
  (set `self.Found` false)
  (for _array_element (`self.Enemies`)
    (if (`|EnumEquality` (`EnemyPawn.AmmoType` _array_element) AmmoType)
      (set `self.Found` true)))
  (return (`self.Found`)))

(fn `CheckForSpawnWeaponAbility`
  (params (B :type "EAmmoType Enum" :default "EAT_HitScan"))
  (returns (Found :type Boolean))
  (set `self.Found` false)
  (for _array_element (`self.WeaponsSpawned`)
    (if (`|EnumEquality` (`WeaponBase.AmmoType` _array_element) B)
      (set `self.Found` true)
      (break)))
  (return (`self.Found`)))

(fn `UserConstructionScript`)