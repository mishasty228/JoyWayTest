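; BP_EnemyBase is a turret enemy that picks its blaster mesh from AmmoType and dies when Health runs out.
; When the player character begins overlapping its sphere, it turns the turret toward them once, with a yaw offset for mesh orientation, and fires.
; Fire implements only Hitscan: a debug-drawn line trace along the turret's negative right vector that passes Damage to a hit player.
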(event `self.ReceiveBeginPlay`
  (bind _turretmesh (`self.TurretMesh`))
  (switch `EAmmoType` (`self.AmmoType`)
    (:`EAT_HitScan`
      (`StaticMeshComponent.SetStaticMesh` _turretmesh "/Game/JoyWay/Core/WeaponModels/FBX_format/blasterE.blasterE"))
    (:`EAT_Projectile`
      (`StaticMeshComponent.SetStaticMesh` _turretmesh "/Game/JoyWay/Core/WeaponModels/FBX_format/blasterA.blasterA"))
    (:`EAT_Bombing`
      (`StaticMeshComponent.SetStaticMesh` _turretmesh "/Game/JoyWay/Core/WeaponModels/FBX_format/blasterD.blasterD"))
    (:`EAT_None`
      (`StaticMeshComponent.SetStaticMesh` _turretmesh null))))

(event `self.Sphere.OnComponentBeginOverlap`
  (params (OverlappedComponent :type "PrimitiveComponent Object Reference") (OtherActor :type "Actor Object Reference") (OtherComp :type "PrimitiveComponent Object Reference") (OtherBodyIndex :type Integer) (bFromSweep :type Boolean) (SweepResult :type "HitResult Structure (by ref)"))
  (bind _turretmesh (`self.TurretMesh`))
  (bind _asbp_joy_way_test_character (cast `/Game/JoyWay/Core/GameplayDefaults/BP_JoyWayTestCharacter` OtherActor))
  (bind (_returnvalue_roll _returnvalue_pitch _returnvalue_yaw) (`KismetMathLibrary.BreakRotator` (`KismetMathLibrary.FindLookAtRotation` (`SceneComponent.K2_GetComponentLocation` _turretmesh) (`self.K2_GetActorLocation` _asbp_joy_way_test_character))))
  (`SceneComponent.K2_SetWorldRotation` _turretmesh (`KismetMathLibrary.MakeRotator` _returnvalue_roll _returnvalue_pitch (- _returnvalue_yaw -90.0)) false false)
  (`self.Fire`))

(fn `Die`
  (`self.K2_DestroyActor`))

(fn `Fire`
  (bind _returnvalue (`SceneComponent.K2_GetComponentLocation` (`self.Scene`)))
  (switch `EAmmoType` (`self.AmmoType`)
    (:`EAT_HitScan`
      (bind _outhit (`KismetSystemLibrary.LineTraceSingle` :`Start` _returnvalue :`End` (+ _returnvalue (* (`SceneComponent.GetRightVector` (`self.TurretMesh`)) -3000.0)) :`TraceChannel` "TraceTypeQuery1" :`DrawDebugType` "ForDuration"))
      (bind _asbp_joy_way_test_character (cast `/Game/JoyWay/Core/GameplayDefaults/BP_JoyWayTestCharacter` (`.HitActor` (`GameplayStatics.BreakHitResult` _outhit))))
      (`JoyWayTestCharacter.GetDamage` _asbp_joy_way_test_character (`self.Damage`)))))

(fn `getDamage`
  (params (Damage :type "Float (double-precision)"))
  (bind _output_get (set `self.Health` (- (`self.Health`) Damage)))
  (if (<= _output_get 0.0)
    (`self.Die`)))

(fn `UserConstructionScript`)