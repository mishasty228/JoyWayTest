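; BP_Bomb is a projectile that deals radial damage on impact and destroys itself shortly afterwards or when its lifetime expires.
; On mesh hit, it loops over actors overlapping Collision, damaging BP_EnemyBase instances matching TargetType within Range.
; For other overlaps, it tests the hit actor, rather than the loop element, as a player target, so damage can repeat.
; Damage scales with distance over Range, increasing toward the edge.
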(event `self.ReceiveBeginPlay`
  (`KismetSystemLibrary.Delay` 2.0)
  (`self.K2_DestroyActor`))

(event `self.Mesh.OnComponentHit`
  (params (HitComponent :type "PrimitiveComponent Object Reference") (OtherActor :type "Actor Object Reference") (OtherComp :type "PrimitiveComponent Object Reference") (NormalImpulse :type "Vector Structure") (Hit :type "HitResult Structure (by ref)"))
  (bind _targettype (`self.TargetType`))
  (bind _range (`self.Range`))
  (bind _range_2 (`self.Range`))
  (bind _returnvalue (`SceneComponent.K2_GetComponentLocation` (`self.Mesh`)))
  (for _array_element (`PrimitiveComponent.GetOverlappingActors` (`self.Collision`) "/Script/Engine.Actor")
    (bind _asbp_enemy_base (cast `/Game/JoyWay/Core/Enemy/BP_EnemyBase` _array_element)
      (:`then`
        (if (== (`GameplayStatics.GetObjectClass` _asbp_enemy_base) _targettype)
          (bind _returnvalue_2 (`KismetMathLibrary.VSize` (- (`SceneComponent.K2_GetComponentLocation` (`EnemyPawn.StandMesh` _asbp_enemy_base)) _returnvalue)))
          (if (<= _returnvalue_2 _range_2)
            (`/Game/JoyWay/Core/Enemy/BP_EnemyBase.getDamage` _asbp_enemy_base (* (/ _returnvalue_2 _range_2) (`self.Damage`))))
          (else
            (bind _asbp_joy_way_test_character (cast `/Game/JoyWay/Core/GameplayDefaults/BP_JoyWayTestCharacter` OtherActor :!label _label))
            (if (== (`GameplayStatics.GetObjectClass` _asbp_joy_way_test_character) _targettype)
              (bind _returnvalue_3 (`KismetMathLibrary.VSize` (- (`SceneComponent.K2_GetComponentLocation` (`Character.Mesh` _asbp_joy_way_test_character)) _returnvalue)))
              (if (<= _returnvalue_3 _range)
                (`JoyWayTestCharacter.GetDamage` _asbp_joy_way_test_character (* (/ _returnvalue_3 _range) (`self.Damage`))))))))
      (:`CastFailed`
        (goto _label))))
  (`KismetSystemLibrary.Delay` 0.2)
  (`self.K2_DestroyActor`))

(fn `UserConstructionScript`)