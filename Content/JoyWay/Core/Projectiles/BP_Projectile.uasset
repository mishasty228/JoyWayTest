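; Base-named projectile actor that damages either enemies or the player character on impact, depending on its TargetType.
; On a Mesh hit it casts the other actor to BP_EnemyBase or BP_JoyWayTestCharacter and calls GetDamage with Damage only on an exact class match, so subclasses of TargetType are not damaged.
; It destroys itself after hitting either kind of character, matched or not, but hits on any other actor leave it alive.
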(event `self.Mesh.OnComponentHit`
  (params (HitComponent :type "PrimitiveComponent Object Reference") (OtherActor :type "Actor Object Reference") (OtherComp :type "PrimitiveComponent Object Reference") (NormalImpulse :type "Vector Structure") (Hit :type "HitResult Structure (by ref)"))
  (bind _targettype (`self.TargetType`))
  (bind _damage (`self.Damage`))
  (bind _asbp_enemy_base (cast `/Game/JoyWay/Core/Enemy/BP_EnemyBase` OtherActor)
    (:`then`
      (if (== (`GameplayStatics.GetObjectClass` _asbp_enemy_base) _targettype)
        (`/Game/JoyWay/Core/Enemy/BP_EnemyBase.getDamage` _asbp_enemy_base _damage)))
    (:`CastFailed`
      (bind _asbp_joy_way_test_character (cast `/Game/JoyWay/Core/GameplayDefaults/BP_JoyWayTestCharacter` OtherActor))
      (if (== (`GameplayStatics.GetObjectClass` _asbp_joy_way_test_character) _targettype)
        (`JoyWayTestCharacter.GetDamage` _asbp_joy_way_test_character _damage))))
  (`self.K2_DestroyActor`))

(fn `UserConstructionScript`)